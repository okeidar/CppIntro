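; BP_SimpleTurret is a turret that fires projectiles at a target detected by its sphere trigger, limited by an ammo supply.
; The most recent actor to enter the sphere becomes the target, which is cleared when that actor leaves.
; Shoot extends the parent's logic with a short delay, spawns a projectile aimed at the target, then subtracts ammo.
; CanShoot adds an ammo check to the parent's, and a TextRender displays ammo changes.
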(event OnValueChanged(Ammo)
  (params (NewValue :type Float%20%28single-precision%29))
  (Rendering|Components|TextRender|SetText (Variables|Default|GetTextRender) (Utilities|Text|FormatText "{0} / {1}" NewValue (Class|ResourceComponent|GetMaxValue (Variables|Default|GetAmmo)))))

(event OnComponentBeginOverlap(Sphere)
  (params (OverlappedComponent :type Primitive%20Component%20Object%20Reference) (OtherActor :type Actor%20Object%20Reference) (OtherComp :type Primitive%20Component%20Object%20Reference) (OtherBodyIndex :type Integer) (bFromSweep :type Boolean) (SweepResult :type Hit%20Result%20Structure%20%28by%20ref%29))
  (Variables|Default|SetTarget OtherActor))

(event OnComponentEndOverlap(Sphere)
  (params (OverlappedComponent :type Primitive%20Component%20Object%20Reference) (OtherActor :type Actor%20Object%20Reference) (OtherComp :type Primitive%20Component%20Object%20Reference) (OtherBodyIndex :type Integer))
  (if (== OtherActor (Variables|Default|GetTarget))
    (Variables|Default|SetTarget 0)))

(event EventShoot
  (bind _shootingpoint1 (Variables|Default|GetShootingPoint1))
  (bind _returnvalue (Transformation|GetWorldLocation _shootingpoint1))
  (|CallParentFunction)
  (Utilities|FlowControl|Delay 0.2)
  (Game|SpawnActorfromClass (Variables|Default|GetProjectileClass) (Math|Transform|MakeTransform _returnvalue (Math|Rotator|FindLookatRotation _returnvalue (Transformation|GetActorLocation (Variables|Default|GetTarget))) "1.000000,1.000000,1.000000") "AlwaysSpawn" 0 0)
  (Class|ResourceComponent|SubtractValue (Variables|Default|GetAmmo) 1.0))

(fn ConstructionScript)

(fn CanShoot
  (bind _returnvalue (|CallParentFunction))
  (return (and _returnvalue (> (Class|ResourceComponent|GetCurrentValue (Variables|Default|GetAmmo)) 0.0))))